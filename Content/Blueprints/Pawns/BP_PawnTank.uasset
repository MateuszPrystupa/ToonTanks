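; BP_PawnTank is a player tank pawn with a movement smoke trail, a fire input and a health value.
; W shows and hides the trail component after short delays, and it starts hidden at BeginPlay, where health is initialized and printed.
; Left mouse calls Shot, which plays a sound and has a validity-checked bullet destroy.
; The bullet spawn logic is disconnected, so firing creates no projectile here.
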(event Custom|ChangeComponentVisibilty
  (params (isVisable :type Boolean)))

(event EventBeginPlay
  (Rendering|SetVisibility (Variables|Default|GetP_ProjectileTrail) false false)
  (bind _output_get (Variables|Default|SetPlayerHealth 100))
  (Development|PrintText (Utilities|Text|ToText(Integer) _output_get)))

(event Collision|EventActorBeginOverlap
  (params (OtherActor :type Actor%20Object%20Reference)))

(event EventTick
  (params (DeltaSeconds :type Float%20%28single-precision%29)))

(event Input|KeyboardEvents|W
  (params (Key :type Key%20Structure :default "None"))
  ;[1 1 1] Enable/disable smoke of movement
  (:Pressed
    (Utilities|FlowControl|Delay 0.1)
    (Rendering|SetVisibility (Variables|Default|GetP_ProjectileTrail) true false))
  (:Released
    (Utilities|FlowControl|Delay 0.5)
    (Rendering|SetVisibility (Variables|Default|GetP_ProjectileTrail) false false)))

(event Input|MouseEvents|LeftMouseButton
  (params (Key :type Key%20Structure :default "None"))
  ;[1 1 1] Fire + destroy bullet
  (:Pressed
    (CallFunction|Shot)))

(fn ConstructionScript)

(fn Shot
  (Audio|PlaySound2D "/Game/Assets/Effects/pew_pew-dknight556-1379997159.pew_pew-dknight556-1379997159" 1.0 1.0 0.0 0 0)
  (Utilities|IsValid 0
    (:Is%20Valid
      (Actor|DestroyActor (Variables|Default|GetBP_Bullet)))))